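; BP_Pickups is a collectible actor that adds a point to the player's score and destroys itself when overlapped.
; On any overlap it casts player character 0 to BP_FirstPersonCharacter, without checking the overlapping actor, and increments Score there.
; At five or more points it shows Win_Menu, switches to UI-only input with a visible cursor and disables player input.
; Each pickup also plays a squeak sound.
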(event `self.ReceiveActorBeginOverlap`
  (params (OtherActor :type "Actor Object Reference"))
  (bind _returnvalue (`GameplayStatics.GetPlayerController` 0))
  (bind _asbp_first_person_character (cast `/Game/FirstPerson/Blueprints/BP_FirstPersonCharacter` (`GameplayStatics.GetPlayerCharacter` 0)))
  (bind _score (`/Game/FirstPerson/Blueprints/BP_FirstPersonCharacter.Score` _asbp_first_person_character))
  (set `/Game/FirstPerson/Blueprints/BP_FirstPersonCharacter.Score` (+ _score 1) _asbp_first_person_character)
  (`self.K2_DestroyActor`)
  (`|ExecutionSequence`
    (:`then_0`
      (if (>= _score 5)
        (bind _returnvalue_2 (`|CreateWidget` "/Game/UI/Win_Menu.Win_Menu_C"))
        (`UserWidget.AddToViewport` _returnvalue_2 0)
        (set `PlayerController.bShowMouseCursor` true _returnvalue)
        (`WidgetBlueprintLibrary.SetInputMode_UIOnlyEx` _returnvalue _returnvalue_2)
        (`self.DisableInput` _returnvalue null)))
    (:`then_1`
      (`GameplayStatics.PlaySound2D` "/Game/LevelDesign/sounds/Squeak-Sound-Effect.Squeak-Sound-Effect" 1.0 1.0 0.0 null null))))

(fn `UserConstructionScript`)