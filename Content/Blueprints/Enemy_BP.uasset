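; Enemy character Blueprint that roams the navmesh at random and chases pawns it sees.
; From BeginPlay it moves to a random navigable point within a large radius and picks a new one each time a move succeeds.
; When PawnSensing sees a pawn, it raises walk speed and moves toward that pawn.
; Nothing handles failed moves or lowers the speed again.
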(event `self.ReceiveBeginPlay`
  (`self.Move To Random Location`))

(event `Move To Random Location`
  (bind _randomlocation (`NavigationSystemV1.K2_GetRandomLocationInNavigableRadius` (`self.K2_GetActorLocation`) 15000.0 null null))
  (`|AIMoveTo` self _randomlocation null
    (:`OnSuccess`
      (`self.Move To Random Location`))))

(event `self.PawnSensing.OnSeePawn`
  (params (Pawn :type "Pawn Object Reference"))
  (`|ExecutionSequence`
    (:`then_0`
      (set `CharacterMovementComponent.MaxWalkSpeed` 650.0 (`self.CharacterMovement`)))
    (:`then_1`
      (`|AIMoveTo` self (0.0 0.0 0.0) Pawn))))

(fn `UserConstructionScript`)